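; First-person player character for architectural visualization walkthroughs, supporting mouse, keyboard and touch.
; Axis inputs drive walk and smoothed look, with run and crouch keys, while touch drags rotate the view with clamped pitch.
; Double-click or double-tap traces from the screen, auto-walks to FLOOR-tagged surfaces and spawns a target marker.
; go_to_location teleports behind a camera fade while a timeline eases control rotation; the zoom logic is unwired.
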(event Custom|go_to_location
  (params (Bp_Location :type Bp%20Location%20Object%20Reference))
  ;[0 0 0] GO TO LOCATION
  (Default|Fadein (Variables|Default|GetAs%20Bp%20My%20Player%20Controller) 0.25)
  (Utilities|FlowControl|Delay 0.25)
  (AI|Navigation|StopMovement (Variables|Default|GetAs%20Bp%20My%20Player%20Controller))
  (Utilities|FlowControl|Sequence
    (:then_0
      (Variables|Default|SetReturn%20Value%20Y%20%28Pitch%29_0 (.pitch (Transformation|GetWorldRotation (Variables|Default|GetCineCamera))))
      (Variables|Default|SetReturn%20Value%20Z%20%28Yaw%29 (.yaw (Pawn|GetControlRotation (Variables|Default|GetAs%20Bp%20My%20Player%20Controller) :!class /Script/Engine.Controller)))
      (Transformation|Teleport (Transformation|GetActorLocation Bp_Location) (Transformation|GetActorRotation Bp_Location)))
    (:then_1
      (bind _newtrack_0 (Timeline|Timeline_Location PlayFromStart)
        (:Update
          (Pawn|SetControlRotation (Variables|Default|GetAs%20Bp%20My%20Player%20Controller) (Math|Rotator|MakeRotator 0.0 (Math|Float|Lerp (Variables|Default|GetReturn%20Value%20Y%20%28Pitch%29_0) 0.0 _newtrack_0) (Math|Float|Lerp (Variables|Default|GetReturn%20Value%20Z%20%28Yaw%29) (.yaw (Transformation|GetActorRotation Bp_Location)) _newtrack_0))))))
    (:then_2
      (Components|Movement|StopMovementImmediately (Variables|Character|GetCharacterMovement))
      (Utilities|FlowControl|Delay 0.4)
      (Default|FadeOut (Variables|Default|GetAs%20Bp%20My%20Player%20Controller) 0.5))))

(event EventBeginPlay
  ;[0 0 0] BEGIN
  (Utilities|FlowControl|Sequence
    (:then_0
      (bind _asbp_controller_archvizz (Utilities|Casting|CastToBp_Controller_Archvizz (Game|GetPlayerController 0)))
      (Variables|Default|SetAs%20Bp%20My%20Player%20Controller _asbp_controller_archvizz))
    (:then_1
      (bind _loading (Timeline|Timeline PlayFromStart)
        (:Update
          (Variables|Default|SetLoading _loading))))))

(event Input|AxisEvents|InputAxisMoveRight
  (params (AxisValue :type Float%20%28single-precision%29))
  (bind _speed (Variables|Default|Getspeed))
  (bind _returnvalue (* AxisValue _speed))
  ;[0 0 0] MOVEMENT
  (Pawn|Input|AddMovementInput (Transformation|GetActorRightVector) (Math|Float|SelectFloat (* _returnvalue 3.0) _returnvalue (Variables|Default|GetisRun)) false))

(event Input|AxisEvents|InputAxisMoveForward
  (params (AxisValue :type Float%20%28single-precision%29))
  (bind _speed (Variables|Default|Getspeed))
  (bind _returnvalue (* AxisValue _speed))
  ;[0 0 0] MOVEMENT
  (Pawn|Input|AddMovementInput (Transformation|GetActorForwardVector) (Math|Float|SelectFloat (* _returnvalue 3.0) _returnvalue (Variables|Default|GetisRun)) false))

(event Input|AxisEvents|InputAxisLookUpRate
  (params (AxisValue :type Float%20%28single-precision%29))
  ;[0 0 0] PAN CHARACTER
  (if (not (Variables|Default|GetIs_Tactil))
    (bind _output_get (Variables|Default|SetCurrentY (Math|Interpolation|FInterpTo (Variables|Default|GetCurrentY) (* (* AxisValue (Variables|Default|GetMouseMultiply)) -1.0) (Utilities|Time|GetWorldDeltaSeconds) 2e+01)))
    (Pawn|Input|AddControllerPitchInput _output_get)))

(event Input|AxisEvents|InputAxisTurnRate
  (params (AxisValue :type Float%20%28single-precision%29))
  ;[0 0 0] PAN CHARACTER
  (if (not (Variables|Default|GetIs_Tactil))
    (bind _output_get (Variables|Default|SetCurrentX (Math|Interpolation|FInterpTo (Variables|Default|GetCurrentX) (* AxisValue (Variables|Default|GetMouseMultiply)) (Utilities|Time|GetWorldDeltaSeconds) 2e+01)))
    (Pawn|Input|AddControllerYawInput _output_get)))

(event Input|MouseEvents|RightMouseButton
  (params (Key :type Key%20Structure))
  ;[0 0 0] ZOOM
)

(event Input|KeyboardEvents|LeftShift
  (params (Key :type Key%20Structure))
  ;[0 0 0] RUN
  (:Pressed
    (Variables|Default|SetisRun true))
  (:Released
    (Variables|Default|SetisRun false)))

(event Input|MouseEvents|LeftMouseButton
  (params (Key :type Key%20Structure))
  ;[0 0 0] MOUSE / TOUCH ACTION
  (:Pressed
    (if (not (Variables|/Game/Blueprint/Gamemode/Bp_Controller_Archvizz.Bp_Controller_Archvizz_C|Getcinematics (Variables|Default|GetAs%20Bp%20My%20Player%20Controller)))
      (Variables|Default|SetMouseMultiply -0.4)
      (Variables|/Script/Engine.PlayerController|SetbShowMouseCursor (Game|GetPlayerController 0) true)
      (Variables|Default|SetIs_Tactil false)
      (Utilities|DoubleClick
        (:Double
          (Variables|Default|SetScreen%20X (.x (stale Input|TouchEvents|InputTouch Location)))
          (Variables|Default|SetScreen%20Y (.y (stale Input|TouchEvents|InputTouch Location)))
          (bind (_location _is_floor) (CallFunction|GetClickTouchLocation))
          (if _is_floor
            (CallFunction|SimpleMoveLocation _location _is_floor)))))))

(event Input|KeyboardEvents|LeftCtrl
  (params (Key :type Key%20Structure))
  (bind _as_bp_my_player_controller (Variables|Default|GetAs%20Bp%20My%20Player%20Controller))
  (bind _canclick (Variables|/Game/Blueprint/Gamemode/Bp_Controller_Archvizz.Bp_Controller_Archvizz_C|GetCanClick _as_bp_my_player_controller))
  ;[0 0 0] CROUCH
  (:Pressed
    (if _canclick
      (Character|Crouch)))
  (:Released
    (if _canclick
      (Character|UnCrouch))))

(event Input|TouchEvents|InputTouch
  (params (Location :type Vector) (FingerIndex :type ETouchIndex%20Enum))
  (bind _returnvalue (Game|GetPlayerController 0))
  (bind _as_bp_my_player_controller (Variables|Default|GetAs%20Bp%20My%20Player%20Controller))
  (bind (_locationx _locationy _biscurrentlypressed) (Class|PlayerController|GetInputTouchState _returnvalue "Touch1"))
  (bind _cinematics (Variables|/Game/Blueprint/Gamemode/Bp_Controller_Archvizz.Bp_Controller_Archvizz_C|Getcinematics _as_bp_my_player_controller))
  ;[0 0 0] MOUSE / TOUCH ACTION
  (:Pressed
    (if (not _cinematics)
      (Variables|Default|SetMouseMultiply 0.4)
      (Utilities|FlowControl|Sequence
        (:then_0
          (Variables|/Script/Engine.PlayerController|SetbShowMouseCursor (Game|GetPlayerController 0) false)
          (Variables|Default|SetIs_Tactil true)
          (Utilities|DoubleClick
            (:Double
              (Variables|Default|SetScreen%20X (.x Location))
              (Variables|Default|SetScreen%20Y (.y Location))
              (bind (_location _is_floor) (CallFunction|GetClickTouchLocation))
              (if _is_floor
                (CallFunction|SimpleMoveLocation _location _is_floor)))))
        (:then_1
          (Variables|Default|SetTouch_Hold true)
          (Variables|Default|SetTouch_Location_Previous (Math|Vector2D|MakeVector2D _locationx _locationy) :!label _label)))))
  (:Released
    (if (not _cinematics)
      (Utilities|FlowControl|Sequence
        (:then_0
          (if (Variables|Default|GetTouch_Hold)
            (Variables|Default|SetTouch_Hold false)))
        (:then_1
          (goto _label)))))
  (:Moved
    (if (not _cinematics)
      (if _biscurrentlypressed
        (CallFunction|TouchRotation _locationx _locationy)))))

(fn ConstructionScript)

(fn GetClickTouchLocation
  (bind _returnvalue (Game|GetPlayerController 0))
  (bind _is_tactil (Variables|Default|GetIs_Tactil))
  (bind _screen_y (Variables|Default|GetScreen%20Y))
  (bind _screen_x (Variables|Default|GetScreen%20X))
  (bind (_worldlocation _worlddirection) (Game|Player|ConvertMouseLocationToWorldSpace _returnvalue))
  (bind (_worldlocation_2 _worlddirection_2) (Class|PlayerController|DeprojectScreenPositiontoWorld _returnvalue _screen_x _screen_y))
  (bind (_outhit _returnvalue_2) (Collision|LineTraceByChannel (Math|Vector|SelectVector _worldlocation_2 _worldlocation _is_tactil) (+ (Math|Vector|SelectVector _worldlocation_2 _worldlocation _is_tactil) (* (Math|Vector|SelectVector _worlddirection_2 _worlddirection _is_tactil) (Math|Conversions|ToVector(Float) 2.5e+03))) "TraceTypeQuery1" true 0 "ForDuration" true "(R=1.000000,G=0.000000,B=0.000000,A=1.000000)" "(R=0.000000,G=1.000000,B=0.000000,A=1.000000)" 2.0))
  (if _returnvalue_2
    (return (.Location (Collision|BreakHitResult _outhit)) (Actor|ActorHasTag (.HitActor (Collision|BreakHitResult _outhit)) "FLOOR"))))

(fn SimpleMoveLocation
  (params (Location :type Vector) (Is%20Floor :type Boolean))
  (if Is%20Floor
    (AI|Navigation|SimpleMovetoLocation (Game|GetPlayerController 0) Location)
    (Game|SpawnActorfromClass "/Game/Blueprint/Character/Bp_TarguetPlayer.Bp_TarguetPlayer_C" (Math|Transform|MakeTransform Location "0, 0, 0" "1.000000,1.000000,1.000000") "Undefined" "OverrideRootScale" 0 0)
    (else
      (Development|PrintString "NO FLOOR" true true "(R=0.000000,G=0.660000,B=1.000000,A=1.000000)" 5.0)))
  (return))

(fn TouchRotation
  (params (Location_X :type Float%20%28double-precision%29) (Location_Y :type Float%20%28double-precision%29))
  (bind _returnvalue (Pawn|GetControlRotation :!class /Script/Engine.Pawn))
  (Variables|Default|SetTouch_Location_Current (Math|Vector2D|MakeVector2D Location_X Location_Y))
  (Pawn|SetControlRotation (Game|GetPlayerController 0) (Math|Rotator|MakeRotator 0.0 (Math|Float|ClampAngle (+ (* (* (- (/ (.y (Variables|Default|GetTouch_Location_Current)) (.y (Variables|Default|GetTouch_Location_Previous))) 1.0) -1.0) -75.0) (.pitch _returnvalue)) (Variables|Default|GetPitchLimit_Min) (Variables|Default|GetPitchLimit_Max)) (+ (* (- (/ (.x (Variables|Default|GetTouch_Location_Current)) (.x (Variables|Default|GetTouch_Location_Previous))) 1.0) -75.0) (.yaw _returnvalue))))
  (Variables|Default|SetTouch_Location_Previous (Math|Vector2D|MakeVector2D (.x (Variables|Default|GetTouch_Location_Current)) (.y (Variables|Default|GetTouch_Location_Current)))))