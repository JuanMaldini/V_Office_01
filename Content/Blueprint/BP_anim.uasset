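; BP_anim is a door actor that opens and closes by playing a Level Sequence forward or in reverse.
; Box overlap begin plays the sequence forward, while overlap end and BeginPlay play it in reverse.
; Each move creates a new sequence player.
; A separate move-door-editor event, apparently for editor use, toggles direction with IsOpen and destroys the spawned sequence actor immediately after starting playback.
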(event OnComponentBeginOverlap(Box)
  (params (OverlappedComponent :type Primitive%20Component%20Object%20Reference) (OtherActor :type Actor%20Object%20Reference) (OtherComp :type Primitive%20Component%20Object%20Reference) (OtherBodyIndex :type Integer) (bFromSweep :type Boolean) (SweepResult :type Hit%20Result%20Structure%20%28by%20ref%29))
  (CallFunction|Move-door true))

(event OnComponentEndOverlap(Box)
  (params (OverlappedComponent :type Primitive%20Component%20Object%20Reference) (OtherActor :type Actor%20Object%20Reference) (OtherComp :type Primitive%20Component%20Object%20Reference) (OtherBodyIndex :type Integer))
  (CallFunction|Move-door false))

(event Custom|move-door-editor
  (bind (_outactor _returnvalue) (Sequencer|Player|CreateLevelSequencePlayer (Variables|Default|GetLevel%20Sequence)))
  (if (Variables|Default|GetisOpen)
    (Class|MovieSceneSequencePlayer|PlayReverse _returnvalue)
    (Variables|Default|SetisOpen false)
    (else
      (Sequencer|Player|Play _returnvalue :!class /Script/MovieScene.MovieSceneSequencePlayer)
      (Variables|Default|SetisOpen true)))
  (Actor|DestroyActor _outactor))

(event Custom|move-door
  (params (forward :type Boolean))
  (bind _returnvalue (Sequencer|Player|CreateLevelSequencePlayer (Variables|Default|GetLevel%20Sequence)))
  (if forward
    (Sequencer|Player|Play _returnvalue :!class /Script/MovieScene.MovieSceneSequencePlayer)
    (else
      (Class|MovieSceneSequencePlayer|PlayReverse _returnvalue))))

(event EventBeginPlay
  (CallFunction|Move-door false))

(fn ConstructionScript)