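; BP_Switchable is a Blueprint that switches its StaticMesh component between the entries of a Mesh map.
; Each map key supplies the mesh and the value at the same position supplies that mesh's relative transform.
; The construction script calls SetIndex to apply the entry at the stored Index, while SetIndexSend applies an entry from an index passed in.
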(event Custom|set%20index%20send
  (params (index :type Integer))
  (bind _mesh (Variables|Default|Getmesh))
  (bind _keys (Utilities|Map|Keys _mesh))
  (Components|StaticMesh|SetStaticMesh (Variables|Default|GetStaticMesh) (Utilities|Array|Get(acopy) _keys index))
  (bind _values (Utilities|Map|Values _mesh))
  (Transformation|SetRelativeTransform (Variables|Default|GetStaticMesh) (Utilities|Array|Get(acopy) _values index) false false))

(event Custom|set%20index
  (bind _index (Variables|Default|Getindex))
  (bind _mesh (Variables|Default|Getmesh))
  (bind _keys (Utilities|Map|Keys _mesh))
  (Components|StaticMesh|SetStaticMesh (Variables|Default|GetStaticMesh) (Utilities|Array|Get(acopy) _keys _index))
  (bind _values (Utilities|Map|Values _mesh))
  (Transformation|SetRelativeTransform (Variables|Default|GetStaticMesh) (Utilities|Array|Get(acopy) _values _index) false false))

(fn ConstructionScript
  (CallFunction|SetIndex))