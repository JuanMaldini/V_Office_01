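; Player controller for an architectural visualization level that sets up the menu, input and presentation on start.
; BeginPlay runs a list of console commands, creates the W_Menu widget with game-and-UI input, optionally loops the master cinematic, and fades the camera from black.
; Events swap the sunny and night streamed levels and push a chair variant index to all cached BP_Switchable actors.
; The R key restarts the current level.
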(event Custom|restart_level
  ;[0 0 0] RESTART LEVEL
  (Development|PrintString "Restart Level")
  (Utilities|FlowControl|Delay 1.0)
  (bind _returnvalue (Game|GetCurrentLevelName true))
  (Game|OpenLevel(byName) (Utilities|String|StringToName _returnvalue)))

(event Custom|make_ui
  ;[0 0 0] CREATE UI
  (bind _returnvalue (UserInterface|CreateWidget "/Game/UI/W_Menu.W_Menu_C"))
  (bind _output_get (Variables|Default|SetW_Menu _returnvalue))
  (UserInterface|Viewport|AddtoViewport _output_get 0))

(event Custom|initial_cinematics_event
  ;[0 0 0] MAKE CINEMATICS
  (bind _returnvalue (Sequencer|Player|CreateLevelSequencePlayer "/Game/SEQ/Sequences/SEQ_Master.SEQ_Master"))
  (bind _output_get (Variables|Default|Set%20Cinematics _returnvalue))
  (Class|MovieSceneSequencePlayer|PlayLooping _output_get -1))

(event Custom|make_input
  ;[0 0 0] MAKE INPUT
  (Input|SetInputModeGameandUI self (Variables|Default|GetW_Menu) "DoNotLock" false true))

(event Custom|fade_in
  (params (Duration :type Float%20%28single-precision%29))
  ;[0 0 0] MAKE FADE IN
  (CameraFades|StartCameraFade :self (Game|GetPlayerCameraManager 0) :ToAlpha 1.0 :Duration Duration :bShouldFadeAudio true :bHoldWhenFinished true))

(event Custom|fade_out
  (params (Duration :type Float%20%28single-precision%29))
  ;[0 0 0] MAKE FADE OUT
  (CameraFades|StartCameraFade :self (Game|GetPlayerCameraManager 0) :FromAlpha 1.0 :Duration Duration :bShouldFadeAudio true :bHoldWhenFinished true))

(event Custom|Daytime
  (params (Make%20day :type Boolean))
  ;[0 0 0] DAYTIME - LEVEL STREAMING
  (if Make%20day
    (Class|GameplayStatics|UnloadStreamLevelbySoftObjectPtr "/Game/Level/L_Night.L_Night" true)
    (Utilities|FlowControl|Delay 0.2)
    (Class|GameplayStatics|LoadStreamLevelbySoftObjectPtr "/Game/Level/L_Sunny.L_Sunny" true true)
    (else
      (Class|GameplayStatics|UnloadStreamLevelbySoftObjectPtr "/Game/Level/L_Sunny.L_Sunny" true)
      (Utilities|FlowControl|Delay 0.2)
      (Class|GameplayStatics|LoadStreamLevelbySoftObjectPtr "/Game/Level/L_Night.L_Night" true true))))

(event Custom|create-chairange
  (params (index :type Integer))
  (for _array_element (Variables|Default|GetBP_Switchables)
    (Default|SetIndexSend _array_element index)))

(event EventBeginPlay
  (Utilities|FlowControl|Sequence
    (:then_0
      (for _array_element (Variables|Default|GetCommand)
        (Development|ExecuteConsoleCommand _array_element 0)))
    (:then_1
      (CallFunction|MakeUI)
      (CallFunction|MakeInput))
    (:then_2
      (if (Variables|Default|Getcinematics)
        (CallFunction|InitialCinematicsEvent)))
    (:then_3
      (Class|PlayerCameraManager|SetManualCameraFade :self (Game|GetPlayerCameraManager 0) :InFadeAmount 1.0 :bInFadeAudio true)
      (Utilities|FlowControl|Delay 1.0)
      (CallFunction|FadeOut 1.0))
    (:then_4)
    (:then_5
      (bind _outactors (Actor|GetAllActorsOfClass "/Game/Blueprint/BP_Switchable.BP_Switchable_C"))
      (for _array_element_2 _outactors
        (Utilities|Array|AddUnique (Variables|Default|GetBP_Switchables) _array_element_2)))))

(event Input|KeyboardEvents|R
  (params (Key :type Key%20Structure :default "None"))
  ;[0 0 0] RESTART
  (:Pressed
    (CallFunction|RestartLevel)))

(fn ConstructionScript)