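; BP_SetupComps is a Blueprint that dresses a computer setup with keyboard, screen and mouse meshes.
; Its construction script runs three sequenced loops over the SmKeyboard, SmScreen and SmMouse collections, assigning each entry's static mesh to the matching component.
; Each loop overwrites the same component on every pass, so the last entry in each collection is the mesh that remains.
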(fn ConstructionScript
  (Utilities|FlowControl|Sequence
    (:then_0
      (for _array_element (Variables|Default|Getsm_keyboard)
        (Components|StaticMesh|SetStaticMesh (Variables|Default|Getkeyboard) (.StaticMesh (Utilities|Struct|Breakstruct-smtr _array_element)))))
    (:then_1
      (for _array_element_2 (Variables|Default|Getsm_screen)
        (Components|StaticMesh|SetStaticMesh (Variables|Default|Getscreen) (.StaticMesh (Utilities|Struct|Breakstruct-smtr _array_element_2)))))
    (:then_2
      (for _array_element_3 (Variables|Default|Getsm_mouse)
        (Components|StaticMesh|SetStaticMesh (Variables|Default|Getmouse) (.StaticMesh (Utilities|Struct|Breakstruct-smtr _array_element_3)))))))